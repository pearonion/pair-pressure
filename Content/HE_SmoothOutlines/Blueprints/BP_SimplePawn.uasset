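; BP_SimplePawn is a pawn that outlines the interactable object its camera is looking at.
; Each tick it traces forward from the camera against static and dynamic world objects, storing any hit actor tagged Interactable and enabling its outline with a fixed stencil value.
; Otherwise it disables the stored actor's outline, but never clears that reference, and switching directly between interactables leaves the previous outline on.
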(event EventTick
  (params (DeltaSeconds :type Float%20%28single-precision%29))
  (bind _camera (Variables|Default|GetCamera))
  (bind _returnvalue (Transformation|GetWorldLocation _camera))
  (bind _outhit (Collision|LineTraceForObjects _returnvalue (+ _returnvalue (* (Math|Vector|GetForwardVector _camera) 1.5e+03)) (Utilities|Array|MakeArray "ObjectTypeQuery1" "ObjectTypeQuery2") false (Utilities|Array|MakeArray self) "None"))
  (if (.bBlockingHit (Collision|BreakHitResult _outhit))
    (if (Actor|ActorHasTag (.HitActor (Collision|BreakHitResult _outhit)) "Interactable")
      (bind _output_get (Variables|Default|SetCurrentInteractable (.HitActor (Collision|BreakHitResult _outhit))))
      (CallFunction|EnableOutline _output_get 64)
      (else
        (bind _currentinteractable (Variables|Default|GetCurrentInteractable :!label _label)
          (:then
            (CallFunction|DisableOutline _currentinteractable))
          (:else))))
    (else
      (goto _label))))

(fn ConstructionScript)