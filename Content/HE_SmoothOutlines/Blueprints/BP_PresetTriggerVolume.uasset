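; BP_PresetTriggerVolume is a trigger actor that showcases an outline preset from the Smooth Outlines pack while something overlaps it.
; Begin overlap on Collision enables the preset's post-process material and a stencil-based outline on the Cube component; end overlap disables both.
; The construction script colors the trigger mesh through a dynamic material instance and sets the text label to the preset's description.
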(event OnComponentBeginOverlap(Collision)
  (params (OverlappedComponent :type Primitive%20Component%20Object%20Reference) (OtherActor :type Actor%20Object%20Reference) (OtherComp :type Primitive%20Component%20Object%20Reference) (OtherBodyIndex :type Integer) (bFromSweep :type Boolean) (SweepResult :type Hit%20Result%20Structure%20%28by%20ref%29))
  (CallFunction|EnablePostProcessVolumeMaterial (Variables|Default|GetOutline%20Preset%20Material))
  (CallFunction|EnableOutlineonComponent (Variables|Default|GetCube) 89))

(event OnComponentEndOverlap(Collision)
  (params (OverlappedComponent :type Primitive%20Component%20Object%20Reference) (OtherActor :type Actor%20Object%20Reference) (OtherComp :type Primitive%20Component%20Object%20Reference) (OtherBodyIndex :type Integer))
  (CallFunction|DisablePostProcessVolumeMaterial)
  (CallFunction|DisableOutlineonComponent (Variables|Default|GetCube)))

(event EventBeginPlay)

(event Collision|EventActorBeginOverlap
  (params (OtherActor :type Actor%20Object%20Reference)))

(event EventTick
  (params (DeltaSeconds :type Float%20%28single-precision%29)))

(fn ConstructionScript
  (bind _returnvalue (Rendering|Material|CreateDynamicMaterialInstance (Variables|Default|GetMesh) 0 "/Game/HE_SmoothOutlines/Materials/Misc/M_FlatColorTrigger.M_FlatColorTrigger" "None" :!class /Script/Engine.PrimitiveComponent))
  (Rendering|Material|SetVectorParameterValue _returnvalue "Color" (Variables|Default|GetColor) :!class /Script/Engine.MaterialInstanceDynamic)
  (Rendering|Components|TextRender|SetText (Variables|Default|GetTextRender) (Variables|Default|GetOutlineDescription)))