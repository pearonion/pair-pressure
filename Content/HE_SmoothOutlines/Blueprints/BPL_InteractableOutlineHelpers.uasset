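; Blueprint function library that toggles custom-depth stencil outlines on interactable actors and components.
; Enable functions set a stencil value and turn on custom depth rendering, while disable functions reset both.
; Actor versions affect only the first StaticMeshComponent found; component versions act on the one passed in.
; Post-process helpers find a PostProcessVolume in the level and replace or clear its entire material blendable list.
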(fn EnableOutline
  (params (Actor :type Actor%20Object%20Reference) (Stencil%20Value :type Integer))
  (bind _returnvalue (Actor|GetComponentbyClass Actor "/Script/Engine.StaticMeshComponent"))
  (Utilities|IsValid _returnvalue
    (:Is%20Valid
      (Rendering|SetCustomDepthStencilValue _returnvalue Stencil%20Value)
      (Rendering|SetRenderCustomDepth _returnvalue true))))

(fn DisableOutline
  (params (Actor :type Actor%20Object%20Reference))
  (bind _returnvalue (Actor|GetComponentbyClass Actor "/Script/Engine.StaticMeshComponent"))
  (Utilities|IsValid _returnvalue
    (:Is%20Valid
      (Rendering|SetCustomDepthStencilValue _returnvalue 0)
      (Rendering|SetRenderCustomDepth _returnvalue false))))

(fn EnablePostProcessVolumeMaterial
  (params (PostProcessMaterial :type Object%20Object%20Reference))
  (bind _returnvalue (Actor|GetActorOfClass 0 "/Script/Engine.PostProcessVolume"))
  (Utilities|Struct|SetmembersinPostProcessSettings (Variables|/Script/Engine.PostProcessVolume|GetSettings _returnvalue) (Utilities|Struct|MakeWeightedBlendables (Utilities|Array|MakeArray (Utilities|Struct|MakeWeightedBlendable 1.0 PostProcessMaterial)))))

(fn DisablePostProcessVolumeMaterial
  (bind _returnvalue (Actor|GetActorOfClass 0 "/Script/Engine.PostProcessVolume"))
  (Utilities|Struct|SetmembersinPostProcessSettings (Variables|/Script/Engine.PostProcessVolume|GetSettings _returnvalue) (Utilities|Struct|MakeWeightedBlendables (Utilities|Array|MakeArray))))

(fn EnableOutlineonComponent
  (params (Component :type Primitive%20Component%20Object%20Reference) (Stencil%20Value :type Integer))
  (Utilities|IsValid Component
    (:Is%20Valid
      (Rendering|SetCustomDepthStencilValue Component Stencil%20Value)
      (Rendering|SetRenderCustomDepth Component true))))

(fn DisableOutlineonComponent
  (params (Compoenent :type Primitive%20Component%20Object%20Reference))
  (Utilities|IsValid Compoenent
    (:Is%20Valid
      (Rendering|SetCustomDepthStencilValue Compoenent 0)
      (Rendering|SetRenderCustomDepth Compoenent false))))