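; BP_MainMenuBootstrap is an actor that brings up the main menu when play begins.
; After a short delay it creates WBP_VNHMainMenu and, if valid, adds it at high Z-order and shows a default hardware cursor.
; It sets UI-only input, then immediately overrides that with Game and UI focused on the widget.
; Print strings trace each step and report a failed widget creation.
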(event EventBeginPlay
  (bind _returnvalue (Game|GetPlayerController 0))
  (Utilities|FlowControl|Delay 0.25)
  (Development|PrintString "MainMenu bootstrap BeginPlay")
  (bind _returnvalue_2 (UserInterface|CreateWidget "/Game/UI/WBP_VNHMainMenu.WBP_VNHMainMenu_C" _returnvalue))
  (Utilities|IsValid _returnvalue_2
    (:Is%20Valid
      (Development|PrintString "MainMenu CreateWidget VALID")
      (UserInterface|Viewport|AddtoViewport _returnvalue_2 5000)
      (Development|PrintString "MainMenu widget AddToViewport complete")
      (Class|WidgetBlueprintLibrary|SetHardwareCursor "Default" "Slate/default-cursor" "(X=0.000000,Y=0.000000)")
      (Variables|/Script/Engine.PlayerController|SetbShowMouseCursor _returnvalue true)
      (Variables|/Script/Engine.PlayerController|SetCurrentMouseCursor _returnvalue "Default")
      (Input|SetInputModeUIOnly _returnvalue _returnvalue_2 "DoNotLock" false)
      (Input|SetInputModeGameandUI _returnvalue _returnvalue_2 "DoNotLock" false false))
    (:Is%20Not%20Valid
      (Development|PrintString "MainMenu CreateWidget INVALID"))))

(event Collision|EventActorBeginOverlap
  (params (OtherActor :type Actor%20Object%20Reference)))

(event EventTick
  (params (DeltaSeconds :type Float%20%28single-precision%29)))

(fn ConstructionScript)