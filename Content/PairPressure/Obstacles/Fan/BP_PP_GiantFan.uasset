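; Giant fan obstacle for PairPressure that spins and pushes actors entering its wind volume.
; A movement component, AlwaysActiveMotion, drives RotatingRoot, while WindVolume detects overlaps.
; On begin overlap, the server sends the other actor a large tether force along the fan's forward vector, once per entry rather than continuously.
; It also exposes an owner player ID and a placement check that always passes.
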(event OnComponentBeginOverlap(WindVolume)
  (params (OverlappedComponent :type Primitive%20Component%20Object%20Reference) (OtherActor :type Actor%20Object%20Reference) (OtherComp :type Primitive%20Component%20Object%20Reference) (OtherBodyIndex :type Integer) (bFromSweep :type Boolean) (SweepResult :type Hit%20Result%20Structure%20%28by%20ref%29))
  (Networking|SwitchHasAuthority
    (:Authority
      (Class|BPIPPTetherEndpoint|ApplyTetherForce(Message) OtherActor (* (Transformation|GetActorForwardVector self) "450000,450000,450000")))))

(event EventBeginPlay
  (Collision|SetCollisionProfileName (Variables|Default|GetWindVolume) "OverlapAllDynamic" true :!class /Script/Engine.PrimitiveComponent)
  (Components|Movement|SetUpdatedComponent (Variables|Default|GetAlwaysActiveMotion) (Variables|Default|GetRotatingRoot)))

(event Collision|EventActorBeginOverlap
  (params (OtherActor :type Actor%20Object%20Reference)))

(event EventTick
  (params (DeltaSeconds :type Float%20%28single-precision%29)))

(fn ConstructionScript)

(fn GetOwnerPlayerId
  (return (Variables|PairPressure|Ownership|GetOwnerPlayerId)))

(fn ValidatePlacement
  (params (ProposedTransform :type Transform))
  (return true))