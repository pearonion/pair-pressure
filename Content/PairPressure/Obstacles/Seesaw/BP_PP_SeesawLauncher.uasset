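; Seesaw obstacle for PairPressure that tilts its platform toward a fixed angle based on which side holds more overlapping actors.
; On Tick, the authority compares the left and right sensor overlap counts and snaps the relative rotation either way, or level on a tie.
; Despite the Launcher name it applies no launch; overlap events are empty.
; It also exposes an owner player ID getter and a placement check that always passes.
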(event OnComponentBeginOverlap(LeftWeightSensor)
  (params (OverlappedComponent :type Primitive%20Component%20Object%20Reference) (OtherActor :type Actor%20Object%20Reference) (OtherComp :type Primitive%20Component%20Object%20Reference) (OtherBodyIndex :type Integer) (bFromSweep :type Boolean) (SweepResult :type Hit%20Result%20Structure%20%28by%20ref%29)))

(event OnComponentEndOverlap(LeftWeightSensor)
  (params (OverlappedComponent :type Primitive%20Component%20Object%20Reference) (OtherActor :type Actor%20Object%20Reference) (OtherComp :type Primitive%20Component%20Object%20Reference) (OtherBodyIndex :type Integer)))

(event OnComponentBeginOverlap(RightWeightSensor)
  (params (OverlappedComponent :type Primitive%20Component%20Object%20Reference) (OtherActor :type Actor%20Object%20Reference) (OtherComp :type Primitive%20Component%20Object%20Reference) (OtherBodyIndex :type Integer) (bFromSweep :type Boolean) (SweepResult :type Hit%20Result%20Structure%20%28by%20ref%29)))

(event OnComponentEndOverlap(RightWeightSensor)
  (params (OverlappedComponent :type Primitive%20Component%20Object%20Reference) (OtherActor :type Actor%20Object%20Reference) (OtherComp :type Primitive%20Component%20Object%20Reference) (OtherBodyIndex :type Integer)))

(event EventBeginPlay
  (Collision|SetCollisionProfileName (Variables|Default|GetLeftWeightSensor) "OverlapAllDynamic" true :!class /Script/Engine.PrimitiveComponent)
  (Collision|SetCollisionProfileName (Variables|Default|GetRightWeightSensor) "OverlapAllDynamic" true :!class /Script/Engine.PrimitiveComponent))

(event Collision|EventActorBeginOverlap
  (params (OtherActor :type Actor%20Object%20Reference)))

(event EventTick
  (params (DeltaSeconds :type Float%20%28single-precision%29))
  (bind _leftweightsensor (Variables|Default|GetLeftWeightSensor))
  (bind _rightweightsensor (Variables|Default|GetRightWeightSensor))
  (bind _platform (Variables|Default|GetPlatform))
  (bind _overlappingactors (Collision|GetOverlappingActors _leftweightsensor 0 :!class /Script/Engine.PrimitiveComponent))
  (bind _overlappingactors_2 (Collision|GetOverlappingActors _rightweightsensor 0 :!class /Script/Engine.PrimitiveComponent))
  (bind _returnvalue (Utilities|Array|Length _overlappingactors))
  (bind _returnvalue_2 (Utilities|Array|Length _overlappingactors_2))
  (if (Ability|HasAuthority) ; Authority-only coordinated seesaw update
    (if (> _returnvalue _returnvalue_2) ; Left occupant count wins
      (Transformation|SetRelativeRotation _platform "12,0,0" false false)
      (elif (> _returnvalue_2 _returnvalue) ; Right occupant count wins; equal counts reset level
        (Transformation|SetRelativeRotation _platform "-12,0,0" false false)
        (else
          (Transformation|SetRelativeRotation _platform "0, 0, 0" false false))))))

(fn ConstructionScript)

(fn GetOwnerPlayerId
  (return (Variables|PairPressure|Ownership|GetOwnerPlayerId)))

(fn ValidatePlacement
  (params (ProposedTransform :type Transform))
  (return true))