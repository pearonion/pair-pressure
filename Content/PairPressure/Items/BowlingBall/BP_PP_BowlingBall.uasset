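; Throwable bowling ball item that launches from the using actor and deals impacts to whatever it hits.
; On primary use it detaches, enables collision and physics, applies a mass-independent impulse along the user's aim direction, then tells the user to drop it.
; On hit, the authority maps impact impulse to a clamped severity and sends it to the other actor with point, normal and itself as instigator.
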(event EventBeginPlay
  (|CallParentFunction) ; This node is disabled and will not be called.\nDrag off pins to build functionality.
)

(event Collision|EventActorBeginOverlap
  (params (OtherActor :type Actor%20Object%20Reference))
  (|CallParentFunction OtherActor) ; This node is disabled and will not be called.\nDrag off pins to build functionality.
)

(event EventTick
  (params (DeltaSeconds :type Float%20%28single-precision%29))
  (|CallParentFunction DeltaSeconds) ; This node is disabled and will not be called.\nDrag off pins to build functionality.
)

(event EventExecutePrimary
  (params (UsingActor :type Actor%20Object%20Reference))
  (bind _self self)
  (bind _returnvalue (Actor|GetComponentbyClass _self "/Script/Engine.StaticMeshComponent"))
  (Transformation|DetachFromActor _self "KeepRelative" "KeepRelative" "KeepRelative")
  (Collision|SetActorEnableCollision _self true)
  (bind _aimdirection (Class|BPIPPItemUser|GetAimData(Message) UsingActor))
  (Physics|SetSimulatePhysics _returnvalue true)
  (Physics|AddImpulse _returnvalue (* _aimdirection "850,850,850") "None" true)
  (Class|BPIPPItemUser|DropItem(Message) UsingActor))

(event Collision|EventHit
  (params (MyComp :type Primitive%20Component%20Object%20Reference) (Other :type Actor%20Object%20Reference) (OtherComp :type Primitive%20Component%20Object%20Reference) (bSelfMoved :type Boolean) (HitLocation :type Vector :default "0, 0, 0") (HitNormal :type Vector :default "0, 0, 0") (NormalImpulse :type Vector :default "0, 0, 0") (Hit :type Hit%20Result%20Structure%20%28by%20ref%29))
  (bind (_bblockinghit _binitialoverlap _time _distance _location _impactpoint _normal _impactnormal) (Collision|BreakHitResult Hit))
  (bind _self self)
  (if (Ability|HasAuthority _self)
    (Class|BPIPPImpactReceiver|ReceiveImpactData(Message) Other (Math|Float|MapRangeClamped (Math|Vector|VectorLength NormalImpulse) 5e+03 6e+04 25.0 1e+02) _impactpoint _impactnormal _self)))

(fn ConstructionScript
  (|CallParentFunction))