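; BP_PP_TrafficCone is a traffic cone item for PairPressure that its user can put down with a primary action.
; ExecutePrimary detaches the cone, re-enables actor collision and turns physics simulation off on its static mesh, so it does not fall under physics.
; It then sends DropItemMessage to the using actor.
; BeginPlay, overlap and Tick are disabled stubs, and construction only calls the parent.
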(event EventBeginPlay
  (|CallParentFunction) ; This node is disabled and will not be called.\nDrag off pins to build functionality.
)

(event Collision|EventActorBeginOverlap
  (params (OtherActor :type Actor%20Object%20Reference))
  (|CallParentFunction OtherActor) ; This node is disabled and will not be called.\nDrag off pins to build functionality.
)

(event EventTick
  (params (DeltaSeconds :type Float%20%28single-precision%29))
  (|CallParentFunction DeltaSeconds) ; This node is disabled and will not be called.\nDrag off pins to build functionality.
)

(event EventExecutePrimary
  (params (UsingActor :type Actor%20Object%20Reference))
  (bind _self self)
  (Transformation|DetachFromActor _self "KeepRelative" "KeepRelative" "KeepRelative")
  (Collision|SetActorEnableCollision _self true)
  (Physics|SetSimulatePhysics (Actor|GetComponentbyClass _self "/Script/Engine.StaticMeshComponent") false)
  (Class|BPIPPItemUser|DropItem(Message) UsingActor))

(fn ConstructionScript
  (|CallParentFunction))