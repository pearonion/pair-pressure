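; BP_PP_Plunger is an item whose primary action pulls whatever the user is aiming at back along the aim line.
; On the authority only, it gets aim data from the using actor through a message and runs a visibility line trace along that direction.
; A hit actor receives a tether-force message with a large fixed force opposite the aim direction, so the target handles its own reaction.
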(event EventBeginPlay
  (|CallParentFunction) ; This node is disabled and will not be called.\nDrag off pins to build functionality.
)

(event Collision|EventActorBeginOverlap
  (params (OtherActor :type Actor%20Object%20Reference))
  (|CallParentFunction OtherActor) ; This node is disabled and will not be called.\nDrag off pins to build functionality.
)

(event EventTick
  (params (DeltaSeconds :type Float%20%28single-precision%29))
  (|CallParentFunction DeltaSeconds) ; This node is disabled and will not be called.\nDrag off pins to build functionality.
)

(event EventExecutePrimary
  (params (UsingActor :type Actor%20Object%20Reference))
  (Networking|SwitchHasAuthority
    (:Authority
      (bind (_aimorigin _aimdirection) (Class|BPIPPItemUser|GetAimData(Message) UsingActor))
      (bind (_outhit _returnvalue) (Collision|LineTraceByChannel _aimorigin (+ _aimorigin (* _aimdirection "2500,2500,2500")) "TraceTypeQuery1" false 0 "None"))
      (if _returnvalue
        (Class|BPIPPTetherEndpoint|ApplyTetherForce(Message) (.HitActor (Collision|BreakHitResult _outhit)) (* _aimdirection "-350000,-350000,-350000"))))))

(fn ConstructionScript
  (|CallParentFunction))