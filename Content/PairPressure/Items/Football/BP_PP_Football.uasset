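; Throwable football item that players can grab, implementing grab, use, grip and prompt queries, mostly gated by ItemEnabled.
; Primary use detaches it, restores collision and physics, launches it along the user's aim with a velocity-change impulse, then tells the user to drop it.
; On hits, the authority maps normal impulse to a clamped severity and sends impact data to the other actor, naming the ball as instigator.
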(event EventBeginPlay
  (|CallParentFunction) ; This node is disabled and will not be called.\nDrag off pins to build functionality.
)

(event Collision|EventActorBeginOverlap
  (params (OtherActor :type Actor%20Object%20Reference))
  (|CallParentFunction OtherActor) ; This node is disabled and will not be called.\nDrag off pins to build functionality.
)

(event EventTick
  (params (DeltaSeconds :type Float%20%28single-precision%29))
  (|CallParentFunction DeltaSeconds) ; This node is disabled and will not be called.\nDrag off pins to build functionality.
)

(event EventExecutePrimary
  (params (UsingActor :type Actor%20Object%20Reference))
  (bind _self self)
  (bind _propmesh (Variables|Default|GetPropMesh))
  (Transformation|DetachFromActor _self "KeepWorld" "KeepWorld" "KeepRelative")
  (Collision|SetActorEnableCollision _self true)
  (bind _aimdirection (Class|BPIPPItemUser|GetAimData(Message) UsingActor))
  (Physics|SetSimulatePhysics _propmesh true)
  (Physics|AddImpulse _propmesh (* _aimdirection "1650,1650,1650") "None" true)
  (Class|BPIPPItemUser|DropItem(Message) UsingActor))

(event Collision|EventHit
  (params (MyComp :type Primitive%20Component%20Object%20Reference) (Other :type Actor%20Object%20Reference) (OtherComp :type Primitive%20Component%20Object%20Reference) (bSelfMoved :type Boolean) (HitLocation :type Vector :default "0, 0, 0") (HitNormal :type Vector :default "0, 0, 0") (NormalImpulse :type Vector :default "0, 0, 0") (Hit :type Hit%20Result%20Structure%20%28by%20ref%29))
  (bind (_bblockinghit _binitialoverlap _time _distance _location _impactpoint _normal _impactnormal) (Collision|BreakHitResult Hit))
  (bind _self self)
  (if (Ability|HasAuthority _self)
    (Class|BPIPPImpactReceiver|ReceiveImpactData(Message) Other (Math|Float|MapRangeClamped (Math|Vector|VectorLength NormalImpulse) 1e+04 9e+04 1e+01 1e+02) _impactpoint _impactnormal _self)))

(fn ConstructionScript
  (|CallParentFunction))

(fn CanGrab
  (params (RequestingActor :type Actor%20Object%20Reference))
  (return (Variables|PairPressure|Item|GetbItemEnabled)))

(fn CanUse
  (params (RequestingActor :type Actor%20Object%20Reference))
  (return (Variables|PairPressure|Item|GetbItemEnabled)))

(fn GetGripPoints
  (return 0))

(fn GetGripResistance
  (return 0.65))

(fn GetHandlingProfile
  (return (Variables|PairPressure|Item|GetHandlingProfile)))

(fn GetPromptPriority
  (return 50))

(fn GetPromptText
  (return "GRAB FOOTBALL"))

(fn IsPromptAvailable
  (params (RequestingActor :type Actor%20Object%20Reference))
  (return (Variables|PairPressure|Item|GetbItemEnabled)))