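; BP_PP_ItemBase is the base item actor for PairPressure, answering grab, use, handling and prompt queries from its own variables.
; A single ItemEnabled flag gates grabbing, use and prompt availability, while GetGripPoints returns no data.
; Its primary action throws the item: it detaches, restores collision, enables mesh physics, applies a mass-independent impulse along the user's aim, then tells the user to drop it.
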(event EventBeginPlay)

(event Collision|EventActorBeginOverlap
  (params (OtherActor :type Actor%20Object%20Reference)))

(event EventTick
  (params (DeltaSeconds :type Float%20%28single-precision%29)))

(event EventExecutePrimary
  (params (UsingActor :type Actor%20Object%20Reference))
  (bind _self self)
  (bind _returnvalue (Actor|GetComponentbyClass _self "/Script/Engine.StaticMeshComponent"))
  (Transformation|DetachFromActor _self "KeepWorld" "KeepWorld" "KeepWorld")
  (Collision|SetActorEnableCollision _self true)
  (bind _aimdirection (Class|BPIPPItemUser|GetAimData(Message) UsingActor))
  (Physics|SetSimulatePhysics _returnvalue true)
  (Physics|AddImpulse _returnvalue (* _aimdirection "1200,1200,1200") "None" true)
  (Class|BPIPPItemUser|DropItem(Message) UsingActor))

(fn ConstructionScript)

(fn CanGrab
  (params (RequestingActor :type Actor%20Object%20Reference))
  (return (Variables|PairPressure|Item|GetbItemEnabled)))

(fn CanUse
  (params (RequestingActor :type Actor%20Object%20Reference))
  (return (Variables|PairPressure|Item|GetbItemEnabled)))

(fn GetGripPoints
  (return 0))

(fn GetGripResistance
  (return (Variables|PairPressure|Item|GetGripResistance)))

(fn GetHandlingProfile
  (return (Variables|PairPressure|Item|GetHandlingProfile)))

(fn GetPromptPriority
  (return (Variables|PairPressure|Item|GetPromptPriority)))

(fn GetPromptText
  (return (Variables|PairPressure|Item|GetPromptText)))

(fn IsPromptAvailable
  (params (RequestingActor :type Actor%20Object%20Reference))
  (return (Variables|PairPressure|Item|GetbItemEnabled)))