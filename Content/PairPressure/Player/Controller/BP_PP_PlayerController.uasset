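; Player controller for Pair Pressure that owns the local player's HUD and switches cursor and input mode by round phase.
; BeginPlay waits briefly, creates the root HUD (an attached variant is switched off) and caches the first round-flow interface actor.
; Every Tick polls that provider, the controlled pawn and tether providers through interface messages, pushing team, item, home, daze, match, round-result and team-matched tether state into the HUD.
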(event EventBeginPlay
  (bind _self self)
  (Utilities|FlowControl|Delay 0.2)
  (if (Pawn|IsLocalController _self)
    (bind _use_attached_hud (Default|UseAttachedHUD _self))
    (bind _returnvalue (UserInterface|CreateWidget (select _use_attached_hud "/Game/PairPressure/UI/HUD/WBP_PP_HUD_Attached.WBP_PP_HUD_Attached_C" "/Game/PairPressure/UI/HUD/WBP_PP_HUD_Root.WBP_PP_HUD_Root_C") _self))
    (Variables|PairPressure|UI|SetPairPressureHUD _returnvalue)
    (bind _returnvalue_2 (UserInterface|Viewport|AddtoPlayerScreen _returnvalue 25))
    (Variables|PairPressure|UI|SetbPairPressureHUDAdded _returnvalue_2)
    (bind _outactors (Actor|GetAllActorswithInterface "/Game/PairPressure/Core/Interfaces/BPI_PP_RoundFlow.BPI_PP_RoundFlow_C"))
    (Variables|PairPressure|UI|SetPairPressureRoundFlowProvider (Utilities|Array|Get(acopy) _outactors))))

(event EventTick
  (params (DeltaSeconds :type Float%20%28single-precision%29))
  (bind _self self)
  (bind _phaseindex (Class|BPIPPRoundFlow|GetRoundPhaseIndex(Message) (Variables|PairPressure|UI|GetPairPressureRoundFlowProvider)))
  (Variables|Default|SetbShowMouseCursor (== _phaseindex 1))
  (if (== _phaseindex 1)
    (Input|SetInputModeGameandUI _self 0 "DoNotLock" true false)
    (PairPressure|UI|RefreshPairPressurePresentation)
    (else
      (Input|SetInputModeGameOnly _self false)
      (PairPressure|UI|RefreshPairPressurePresentation))))

(fn ConstructionScript)

(fn RefreshPairPressurePresentation
  (bind _returnvalue (Pawn|GetControlledPawn))
  (bind _pairpressureroundflowprovider (Variables|PairPressure|UI|GetPairPressureRoundFlowProvider))
  (bind _pairpressurehud (Variables|PairPressure|UI|GetPairPressureHUD))
  (Utilities|FlowControl|Sequence
    (:then_0
      (bind _winningteamid (Class|BPIPPRoundFlow|GetRoundState(Message) _pairpressureroundflowprovider))
      (Class|BPIPPRoundFlow|GetRoundPhaseIndex(Message) _pairpressureroundflowprovider)
      (if (== (stale _team_id) (stale _teamid))
        (Class|BPIPPResultsView|PresentRoundResult(Message) (Variables|PairPressure|UI|GetPairPressureHUD) _winningteamid)))
    (:then_1
      (bind (_partnername _partnerstate _blocalhome _bpartnerhome _bteamfinished) (Class|BPIPPUIDataProvider|GetTeamPresentation(Message) _returnvalue))
      (bind _partner_direction (Class|BPIPPUIDataProvider|GetPartnerDirectionPresentation(Message) _returnvalue))
      (Class|BPIPPPlayerHUDView|PresentTeamStatus(Message) _pairpressurehud _partnername _partnerstate _partner_direction)
      (bind (_dazenormalized _physicalstate _helditemlabel) (Class|BPIPPUIDataProvider|GetPlayerPresentation(Message) _returnvalue))
      (Class|BPIPPPlayerHUDView|PresentItemStatus(Message) _pairpressurehud _helditemlabel)
      (Class|BPIPPPlayerHUDView|PresentHomeStatus(Message) _pairpressurehud _blocalhome _bpartnerhome _bteamfinished)
      (Class|BPIPPPlayerHUDView|PresentDazeStatus(Message) _pairpressurehud _dazenormalized _physicalstate)
      (bind (_current_round _total_rounds _team_one_score _team_two_score _match_complete) (Class|BPIPPRoundFlow|GetMatchState(Message) _pairpressureroundflowprovider))
      (Class|BPIPPResultsView|PresentMatchState(Message) _pairpressurehud _current_round _total_rounds _team_one_score _team_two_score _match_complete)
      (bind _teamid (Class|BPIPPTeamMember|GetTeamId(Message) _returnvalue))
      (bind _outactors (Actor|GetAllActorswithInterface "/Game/PairPressure/Core/Interfaces/BPI_PP_TetherPresentationProvider.BPI_PP_TetherPresentationProvider_C"))
      (for _array_element _outactors
        (bind (_team_id _tension_normalized _current_distance _broken _connected) (Class|BPIPPTetherPresentationProvider|GetTetherPresentation(Message) _array_element))
        (if (== _team_id _teamid)
          (Class|BPIPPPlayerHUDView|PresentTetherStatus(Message) _pairpressurehud _tension_normalized _current_distance _broken _connected))))))

(fn GetHUDWidgetClass
  (return "/Game/PairPressure/UI/HUD/WBP_PP_HUD_Root.WBP_PP_HUD_Root_C"))

(fn UseAttachedHUD
  (return false))