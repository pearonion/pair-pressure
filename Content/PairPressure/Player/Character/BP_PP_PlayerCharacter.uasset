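; Player character for PairPressure, a game of tethered teammate pairs, with item pickup, drop and primary use.
; On BeginPlay the server derives team from PlayerId parity and, after fixed delays, caches a same-team character as partner.
; Tether events apply movement force and update a state label; finish events track home and team-finished flags.
; Interface getters supply partner bearing and team/player presentation data, while many grab, carry and ragdoll queries return placeholder constants.
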(event EventBeginPlay
  (bind _self self)
  (Networking|SwitchHasAuthority :!pinned true ; Server-authoritative team assignment: PlayerState PlayerId modulo 2 yields two alternating teams.
    (:Authority
      (Utilities|FlowControl|Delay 0.2)
      (Variables|PairPressure|Team|SetPairPressureTeamId (Math|Integer|%(Integer) (Variables|/Script/Engine.PlayerState|GetPlayerId (Variables|Default|GetPlayerState)) 2))
      (Utilities|FlowControl|Delay 0.35)
      (bind _outactors (Actor|GetAllActorsOfClass "BP_PP_PlayerCharacter_C"))
      (for _array_element _outactors ; After all pawns exist, find the other actor with the same team id and cache it as partner.
        (if (and (!= _array_element _self) (== (Default|GetTeamId _array_element) (Variables|PairPressure|Team|GetPairPressureTeamId)))
          (Variables|PairPressure|Team|SetPairPressurePartner _array_element)
          (Default|OnTetherReconnected _self _array_element))))))

(event Collision|EventActorBeginOverlap
  (params (OtherActor :type Actor%20Object%20Reference)))

(event EventTick
  (params (DeltaSeconds :type Float%20%28single-precision%29)))

(event EventApplyTetherForce
  (params (Force :type Vector :default "0, 0, 0"))
  (Physics|AddForce (Variables|Character|GetCharacterMovement) Force))

(event EventOnTetherBroken
  (Variables|PairPressure|HUD|SetPairPressurePhysicalStateLabel "TetherBroken"))

(event EventOnTetherReconnected
  (params (PartnerActor :type Actor%20Object%20Reference))
  (Variables|PairPressure|Team|SetPairPressurePartner PartnerActor)
  (Variables|PairPressure|HUD|SetPairPressurePhysicalStateLabel "Active"))

(event EventDropItem
  (Variables|PairPressure|Items|SetPairPressureHeldItem 0))

(event EventSetHomeState
  (params (Home :type Boolean))
  (Variables|PairPressure|Finish|SetbPairPressureHome Home))

(event EventResetFinishState
  (Variables|PairPressure|Finish|SetbPairPressureHome false)
  (Variables|PairPressure|Finish|SetbPairPressureTeamFinished false))

(event EventOnTeamFinished
  (params (TeamId :type Integer))
  (Variables|PairPressure|Finish|SetbPairPressureHome true)
  (Variables|PairPressure|Finish|SetbPairPressureTeamFinished true))

(event Input|KeyboardEvents|E
  (params (Key :type Key%20Structure))
  (bind _self self)
  (:Pressed
    (if (not (Utilities|IsValid (Variables|PairPressure|Items|GetPairPressureHeldItem)))
      (CallFunction|EquipItem _self (Utilities|Array|Get(acopy) (Collision|GetOverlappingActors _self "/Game/PairPressure/Items/Core/BP_PP_ItemBase.BP_PP_ItemBase_C" :!class /Script/Engine.Actor))))))

(event Input|KeyboardEvents|Q
  (params (Key :type Key%20Structure))
  (:Pressed
    (if (Utilities|IsValid (Variables|PairPressure|Items|GetPairPressureHeldItem))
      (Transformation|DetachFromActor (Variables|PairPressure|Items|GetPairPressureHeldItem) "KeepWorld" "KeepWorld" "KeepWorld")
      (Collision|SetActorEnableCollision (Variables|PairPressure|Items|GetPairPressureHeldItem) true)
      (Variables|PairPressure|Items|SetPairPressureHeldItem 0))))

(event Input|MouseEvents|LeftMouseButton
  (params (Key :type Key%20Structure))
  (bind _pairpressurehelditem (Variables|PairPressure|Items|GetPairPressureHeldItem))
  (:Pressed
    (if (Utilities|IsValid _pairpressurehelditem)
      (Class|BPIPPUsableItem|ExecutePrimary(Message) _pairpressurehelditem self))))

(fn ConstructionScript)

(fn CanCarry
  (params (RequestedCarrier :type Actor%20Object%20Reference))
  (return false))

(fn CanFinish
  (return true))

(fn CanGrab
  (params (RequestingActor :type Actor%20Object%20Reference))
  (return true))

(fn EquipItem
  (params (ItemActor :type Actor%20Object%20Reference))
  (Variables|PairPressure|Items|SetPairPressureHeldItem ItemActor)
  (Collision|SetActorEnableCollision ItemActor false)
  (Transformation|AttachActorToActor ItemActor self "None" "KeepWorld" "KeepWorld" "KeepWorld" true)
  (return (Utilities|IsValid ItemActor)))

(fn GetAimData
  (bind _self self)
  (return (Transformation|GetActorLocation _self) (Transformation|GetActorForwardVector _self)))

(fn GetCarryCapacity
  (return 1.0))

(fn GetCarryProfiles
  (return 0))

(fn GetDazeNormalized
  (return (Variables|PairPressure|UI|GetPairPressureDazeNormalized)))

(fn GetFinishConnections
  (return 0))

(fn GetGrabOrigin
  (return (Transformation|GetActorLocation)))

(fn GetGripPoints
  (return 0))

(fn GetGripResistance
  (return 1.0))

(fn GetGripStrength
  (return 1.0))

(fn GetHomeState
  (return (Variables|PairPressure|Finish|GetbPairPressureHome)))

(fn GetImpactModifier
  (return 1.0))

(fn GetPartner
  (return (Variables|PairPressure|Team|GetPairPressurePartner)))

(fn GetPartnerDirectionPresentation
  (bind _pairpressurepartner (Variables|PairPressure|Team|GetPairPressurePartner))
  (bind _anchorlocation (Class|BPIPPTetherEndpoint|GetTetherAnchor(Message) _pairpressurepartner))
  (return (Utilities|String|SelectText (Utilities|Text|FormatText "PARTNER BEARING {Bearing} DEG" (Math|Float|Round (.Yaw (Math|Rotator|BreakRotator (Math|Rotator|Delta(Rotator) (Math|Rotator|FindLookatRotation (Transformation|GetActorLocation) _anchorlocation) (Transformation|GetActorRotation)))))) "PARTNER SEARCHING" (Utilities|IsValid _pairpressurepartner))))

(fn GetPhysicalState
  (return (Variables|PairPressure|HUD|GetPairPressurePhysicalStateLabel)))

(fn GetPlayerPresentation
  (return (Variables|PairPressure|UI|GetPairPressureDazeNormalized) (Variables|PairPressure|HUD|GetPairPressurePhysicalStateLabel) (Utilities|String|SelectText "ITEM EQUIPPED" "HANDS FREE" (Utilities|IsValid (Variables|PairPressure|Items|GetPairPressureHeldItem)))))

(fn GetRoundPresentation
  (return "" 0.0))

(fn GetTeamId
  (return (Variables|PairPressure|Team|GetPairPressureTeamId)))

(fn GetTeamPresentation
  (bind _pairpressurepartner (Variables|PairPressure|Team|GetPairPressurePartner))
  (bind _physicalstate (Class|BPIPPUIDataProvider|GetPlayerPresentation(Message) _pairpressurepartner))
  (bind _home (Class|BPIPPTeamMember|GetHomeState(Message) _pairpressurepartner))
  (return (Utilities|Text|ToText(String) (Utilities|GetDisplayName _pairpressurepartner)) _physicalstate (Variables|PairPressure|Finish|GetbPairPressureHome) _home (Variables|PairPressure|Finish|GetbPairPressureTeamFinished)))

(fn GetTetherAnchor
  (return (Transformation|GetActorLocation)))

(fn IsFriendlyto
  (params (OtherActor :type Actor%20Object%20Reference))
  (return false))

(fn IsRagdolled
  (return false))

(fn IsUnconscious
  (return false))

(fn RequestCarry
  (params (CarryTarget :type Actor%20Object%20Reference) (CarryProfile :type Name :default "None"))
  (return false))

(fn RequestGrab
  (params (TargetActor :type Actor%20Object%20Reference))
  (return false))