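; BP_PP_BuildSocket is a course socket where a selected obstacle can be placed, holding one obstacle at a time.
; CommitPlacement records a valid obstacle if the socket is free, but its return re-evaluates that check afterwards, so it yields false even on success.
; GetBuildSocketState exposes ID, occupancy, transform and obstacle, while ResetBuildSocket clears occupancy.
; Prompt functions offer fixed placement text and priority, available only while unoccupied.
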(event EventBeginPlay)

(event Collision|EventActorBeginOverlap
  (params (OtherActor :type Actor%20Object%20Reference)))

(event EventTick
  (params (DeltaSeconds :type Float%20%28single-precision%29)))

(event EventResetBuildSocket
  (Variables|PairPressure|Build|SetOccupyingObstacle 0)
  (Variables|PairPressure|Build|SetbOccupied false))

(fn ConstructionScript)

(fn CommitPlacement
  (params (ObstacleActor :type Object%20Object%20Reference) (BuilderActor :type Object%20Object%20Reference))
  (if (and (Utilities|IsValid ObstacleActor) (not (Variables|PairPressure|Build|GetbOccupied)))
    (Variables|PairPressure|Build|SetOccupyingObstacle ObstacleActor)
    (Variables|PairPressure|Build|SetbOccupied true))
  (return (and (Utilities|IsValid ObstacleActor) (not (Variables|PairPressure|Build|GetbOccupied)))))

(fn GetBuildSocketState
  (return (Variables|PairPressure|Build|GetSocketId) (Variables|PairPressure|Build|GetbOccupied) (Transformation|GetActorTransform) (Variables|PairPressure|Build|GetOccupyingObstacle)))

(fn GetPromptPriority
  (return 50))

(fn GetPromptText
  (return "PLACE SELECTED OBSTACLE"))

(fn IsPromptAvailable
  (params (RequestingActor :type Actor%20Object%20Reference))
  (return (not (Variables|PairPressure|Build|GetbOccupied))))