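; Finish area course module for Pair Pressure races that detects team members reaching the end.
; On server-side trigger overlap, any actor implementing the team member interface fires the FinishAreaEntered dispatcher, regardless of race phase.
; During the Racing phase, it registers the pawn's PlayerState and team ID with the finish tracker component on the GameState.
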(event OnComponentBeginOverlap(RaceTrigger)
  (params (OverlappedComponent :type Primitive%20Component%20Object%20Reference) (OtherActor :type Actor%20Object%20Reference) (OtherComp :type Primitive%20Component%20Object%20Reference) (OtherBodyIndex :type Integer) (bFromSweep :type Boolean) (SweepResult :type Hit%20Result%20Structure%20%28by%20ref%29))
  ;[0.15 0.15 0.15 0.5] think steam achievements and incrementing Stats for things like leaderboards and personal stattracking
  (Networking|SwitchHasAuthority
    (:Authority
      (if (Utilities|DoesObjectImplementInterface OtherActor "/Game/PairPressure/Core/Interfaces/BPI_PP_TeamMember.BPI_PP_TeamMember_C")
        (bind _teamid (Class|BPIPPTeamMember|GetTeamId(Message) OtherActor))
        (Default|CallFinishAreaEntered OtherActor)
        (bind _aspawn (Utilities|Casting|CastToPawn OtherActor))
        (bind _asvnhgame_state (Utilities|Casting|CastToVNHGameState (Game|GetGameState)))
        (bind _astttrace_state_component (Utilities|Casting|CastToTTTRaceStateComponent (Actor|GetComponentbyClass _asvnhgame_state "/Script/VNHSimulator.TTTRaceStateComponent")))
        (switch Utilities|FlowControl|Switch|SwitchonETTTRacePhase (Class|TTTRaceStateComponent|GetRacePhase _astttrace_state_component)
          (:Racing
            (bind _astttfinish_tracker_component (Utilities|Casting|CastToTTTFinishTrackerComponent (Actor|GetComponentbyClass _asvnhgame_state "/Script/VNHSimulator.TTTFinishTrackerComponent")))
            (Class|TTTFinishTrackerComponent|RegisterParticipantFinished _astttfinish_tracker_component _teamid (Variables|/Script/Engine.Pawn|GetPlayerState _aspawn))))))))

(event EventBeginPlay)

(event Collision|EventActorBeginOverlap
  (params (OtherActor :type Actor%20Object%20Reference)))

(event EventTick
  (params (DeltaSeconds :type Float%20%28single-precision%29)))

(fn ConstructionScript)