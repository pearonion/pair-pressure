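; BP_PP_HomeFinishZone is a course finish zone that detects when enough members of one team are home together.
; The first team to enter claims the trigger, and overlaps update each member's home state through interface messages.
; At the required count it fires OnTeamFinished, notifies those players and submits the team ID to BPI_PP_RoundFlow actors.
; It then frees the zone, barring finished teams until ResetFinishZoneState clears them.
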(event OnComponentBeginOverlap(HomeTrigger)
  (params (OverlappedComponent :type Primitive%20Component%20Object%20Reference) (OtherActor :type Actor%20Object%20Reference) (OtherComp :type Primitive%20Component%20Object%20Reference) (OtherBodyIndex :type Integer) (bFromSweep :type Boolean) (SweepResult :type Hit%20Result%20Structure%20%28by%20ref%29))
  (bind _playershome (Variables|PairPressure|Finish|GetPlayersHome))
  (if (Utilities|DoesObjectImplementInterface OtherActor "/Game/PairPressure/Core/Interfaces/BPI_PP_TeamMember.BPI_PP_TeamMember_C")
    (bind _teamid (Class|BPIPPTeamMember|GetTeamId(Message) OtherActor))
    (if (and (or (== (Utilities|Array|Length _playershome) 0) (== (Variables|PairPressure|Finish|GetActiveTeamId) _teamid)) (not (Utilities|Array|ContainsItem (Variables|PairPressure|Finish|GetFinishedTeamIds) _teamid))) ; Only the first team to enter claims the zone; opposing-team actors are ignored.
      (Variables|PairPressure|Finish|SetActiveTeamId _teamid)
      (Utilities|Array|AddUnique _playershome OtherActor)
      (Class|BPIPPFinishParticipant|SetHomeState(Message) OtherActor true)
      (if (and (>= (Utilities|Array|Length _playershome) (Variables|PairPressure|Finish|GetRequiredPlayers)) (not (Variables|PairPressure|Finish|GetbTeamFinished)))
        (Utilities|Array|AddUnique (Variables|PairPressure|Finish|GetFinishedTeamIds) (Variables|PairPressure|Finish|GetActiveTeamId))
        (Variables|PairPressure|Finish|SetbTeamFinished true)
        (Default|CallOnTeamFinished (Variables|PairPressure|Finish|GetActiveTeamId))
        (for _array_element _playershome
          (Class|BPIPPFinishParticipant|OnTeamFinished(Message) _array_element (Variables|PairPressure|Finish|GetActiveTeamId)))
        (bind _outactors (Actor|GetAllActorswithInterface "/Game/PairPressure/Core/Interfaces/BPI_PP_RoundFlow.BPI_PP_RoundFlow_C" :!pinned true)) ; Submit the winner through BPI_PP_RoundFlow; the finish zone does not depend on a concrete director class.
        (for _array_element_2 _outactors
          (Class|BPIPPRoundFlow|SubmitRoundResult(Message) _array_element_2 (Variables|PairPressure|Finish|GetActiveTeamId)))
        (Utilities|Array|Clear (Variables|PairPressure|Finish|GetPlayersHome))
        (Variables|PairPressure|Finish|SetActiveTeamId -1)
        (Variables|PairPressure|Finish|SetbTeamFinished false)))))

(event OnComponentEndOverlap(HomeTrigger)
  (params (OverlappedComponent :type Primitive%20Component%20Object%20Reference) (OtherActor :type Actor%20Object%20Reference) (OtherComp :type Primitive%20Component%20Object%20Reference) (OtherBodyIndex :type Integer))
  (Utilities|Array|RemoveItem (Variables|PairPressure|Finish|GetPlayersHome) OtherActor)
  (Class|BPIPPFinishParticipant|SetHomeState(Message) OtherActor false))

(event EventBeginPlay)

(event Collision|EventActorBeginOverlap
  (params (OtherActor :type Actor%20Object%20Reference)))

(event EventTick
  (params (DeltaSeconds :type Float%20%28single-precision%29)))

(event EventResetFinishZoneState
  (Utilities|Array|Clear (Variables|PairPressure|Finish|GetPlayersHome))
  (Utilities|Array|Clear (Variables|PairPressure|Finish|GetFinishedTeamIds))
  (Variables|PairPressure|Finish|SetActiveTeamId -1)
  (Variables|PairPressure|Finish|SetbTeamFinished false))

(fn ConstructionScript)