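; Round director for PairPressure that cycles build, run and results phases across a two-team, multi-round match.
; Delays sequence build, TTT race countdown and run, resetting participants and finish zones through interfaces.
; An authority-only Tick clock ends runs on timeout and advances rounds after results.
; Submitted finishes record the first team and start a post-finish timer, completing the round and scoring that team once enough teams finish.
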(event Custom|AdvanceToNextRound
  (if (not (Variables|PairPressure|Match|GetbMatchComplete))
    (Variables|PairPressure|Match|SetCurrentRoundNumber (+ (Variables|PairPressure|Match|GetCurrentRoundNumber) 1))
    (PairPressure|Round|StartBuildPhase)
    (Utilities|FlowControl|Delay (Variables|PairPressure|Round|GetBuildDuration))
    (CallFunction|BeginTTTRaceCountdown)
    (Utilities|FlowControl|Delay 3.0)
    (PairPressure|Round|StartRunPhase)))

(event Custom|BeginTTTRaceCountdown
  (bind _asvnhgame_state (Utilities|Casting|CastToVNHGameState (Game|GetGameState)))
  (bind _astttrace_state_component (Utilities|Casting|CastToTTTRaceStateComponent (Actor|GetComponentbyClass _asvnhgame_state "/Script/VNHSimulator.TTTRaceStateComponent")))
  (Class|TTTRaceStateComponent|StartCountdown _astttrace_state_component 3.0))

(event EventBeginPlay
  (PairPressure|Round|StartBuildPhase)
  (Utilities|FlowControl|Delay (Variables|PairPressure|Round|GetBuildDuration))
  (CallFunction|BeginTTTRaceCountdown)
  (Utilities|FlowControl|Delay 3.0)
  (PairPressure|Round|StartRunPhase))

(event Collision|EventActorBeginOverlap
  (params (OtherActor :type Actor%20Object%20Reference)))

(event EventTick
  (params (DeltaSeconds :type Float%20%28single-precision%29))
  (Networking|SwitchHasAuthority :!pinned true ; Only the authority advances the replicated phase clock.
    (:Authority
      (bind _output_get (Variables|PairPressure|Round|SetPhaseTimeRemaining (Math|Float|Max(Float) (- (Variables|PairPressure|Round|GetPhaseTimeRemaining) DeltaSeconds) 0.0)))
      (bind _phaseindex (CallFunction|GetRoundPhaseIndex))
      (if (and (<= _output_get 0.0) (== _phaseindex 2))
        (PairPressure|Round|CompleteRound (Variables|PairPressure|RoundResults|GetFirstWinningTeamId))
        (elif (and (<= _output_get 0.0) (== _phaseindex 3))
          (CallFunction|AdvancetoNextRound))))))

(event EventRequestMatchRestart
  (Networking|SwitchHasAuthority
    (:Authority
      (Variables|PairPressure|Match|SetCurrentRoundNumber 1)
      (Variables|PairPressure|Match|SetTeamOneScore 0)
      (Variables|PairPressure|Match|SetTeamTwoScore 0)
      (Variables|PairPressure|Match|SetbMatchComplete false)
      (Variables|PairPressure|Round|SetWinningTeamId -1)
      (PairPressure|Round|StartBuildPhase)
      (Utilities|FlowControl|Delay (Variables|PairPressure|Round|GetBuildDuration))
      (CallFunction|BeginTTTRaceCountdown)
      (Utilities|FlowControl|Delay 3.0)
      (PairPressure|Round|StartRunPhase))))

(fn ConstructionScript)

(fn StartBuildPhase
  (bind _outactors (Actor|GetAllActorswithInterface "/Game/PairPressure/Core/Interfaces/BPI_PP_BuildFlow.BPI_PP_BuildFlow_C"))
  (for _array_element _outactors
    (Class|BPIPPBuildFlow|ResetBuildState(Message) _array_element))
  (Variables|PairPressure|Round|SetCurrentPhase "NewEnumerator1")
  (Variables|PairPressure|Round|SetPhaseTimeRemaining (Variables|PairPressure|Round|GetBuildDuration))
  (Default|CallOnPhaseChanged "NewEnumerator1"))

(fn StartRunPhase
  (Utilities|Array|Clear (Variables|PairPressure|RoundResults|GetFinishedTeamIds))
  (Variables|PairPressure|RoundResults|SetFirstWinningTeamId -1)
  (bind _outactors (Actor|GetAllActorswithInterface "/Game/PairPressure/Core/Interfaces/BPI_PP_FinishZoneReset.BPI_PP_FinishZoneReset_C"))
  (for _array_element _outactors
    (Class|BPIPPFinishZoneReset|ResetFinishZoneState(Message) _array_element))
  (bind _outactors_2 (Actor|GetAllActorswithInterface "/Game/PairPressure/Core/Interfaces/BPI_PP_FinishParticipant.BPI_PP_FinishParticipant_C"))
  (for _array_element_2 _outactors_2
    (Class|BPIPPFinishParticipant|ResetFinishState(Message) _array_element_2))
  (Variables|PairPressure|Round|SetCurrentPhase "NewEnumerator2")
  (Variables|PairPressure|Round|SetPhaseTimeRemaining (Variables|PairPressure|Round|GetRunDuration))
  (Default|CallOnPhaseChanged "NewEnumerator2"))

(fn CompleteRound
  (params (TeamId :type Integer))
  (Variables|PairPressure|Match|SetTeamOneScore (+ (Variables|PairPressure|Match|GetTeamOneScore) (Math|Integer|SelectInt 1 0 (== TeamId 0))))
  (Variables|PairPressure|Match|SetTeamTwoScore (+ (Variables|PairPressure|Match|GetTeamTwoScore) (Math|Integer|SelectInt 1 0 (== TeamId 1))))
  (Variables|PairPressure|Match|SetbMatchComplete (>= (Variables|PairPressure|Match|GetCurrentRoundNumber) (Variables|PairPressure|Match|GetTotalRounds)))
  (Variables|PairPressure|Round|SetWinningTeamId TeamId)
  (Variables|PairPressure|Round|SetCurrentPhase "NewEnumerator3")
  (Variables|PairPressure|Round|SetPhaseTimeRemaining (Variables|PairPressure|Round|GetResultsDuration))
  (Default|CallOnPhaseChanged "NewEnumerator3")
  (Default|CallOnRoundCompleted TeamId))

(fn GetMatchState
  (return (Variables|PairPressure|Match|GetCurrentRoundNumber) (Variables|PairPressure|Match|GetTotalRounds) (Variables|PairPressure|Match|GetTeamOneScore) (Variables|PairPressure|Match|GetTeamTwoScore) (Variables|PairPressure|Match|GetbMatchComplete)))

(fn GetRoundPhaseIndex
  (return (Math|Conversions|ToInteger(Byte) (Variables|PairPressure|Round|GetCurrentPhase))))

(fn GetRoundState
  (return (Utilities|String|StringToName (Utilities|String|EnumtoString (Variables|PairPressure|Round|GetCurrentPhase))) (Variables|PairPressure|Round|GetPhaseTimeRemaining) (Variables|PairPressure|Round|GetWinningTeamId)))

(fn SubmitRoundResult
  (params (WinningTeamId :type Integer))
  (bind _finishedteamids (Variables|PairPressure|RoundResults|GetFinishedTeamIds))
  (bind _returnvalue (Utilities|Array|ContainsItem _finishedteamids WinningTeamId))
  (bind _returnvalue_2 (not _returnvalue))
  (bind _phaseindex (CallFunction|GetRoundPhaseIndex))
  (if (== _phaseindex 2)
    (if _returnvalue_2
      (Utilities|Array|AddUnique (Variables|PairPressure|RoundResults|GetFinishedTeamIds) WinningTeamId)
      (if (>= (Utilities|Array|Length (Variables|PairPressure|RoundResults|GetFinishedTeamIds)) (Variables|PairPressure|RoundResults|GetTeamsRequired))
        (PairPressure|Round|CompleteRound (Variables|PairPressure|RoundResults|GetFirstWinningTeamId))
        (return true)
        (else
          (Variables|PairPressure|RoundResults|SetFirstWinningTeamId WinningTeamId)
          (Variables|PairPressure|Round|SetPhaseTimeRemaining (Variables|PairPressure|RoundResults|GetPostFirstFinishDuration))
          (return true)))
      (else
        (return _returnvalue_2)))
    (else
      (return false))))