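; Tether actor that links two members of a target team with an elastic, breakable bond.
; Shortly after BeginPlay, the authority finds both endpoints through the team-member interface.
; Tick draws a debug line, pulls endpoints together beyond a soft length, and toggles break and reconnect at separate distances, all via interface messages.
; GetTetherPresentation reports team, normalized tension, distance and connection state.
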(event EventBeginPlay
  (Networking|SwitchHasAuthority
    (:Authority
      (Utilities|FlowControl|Delay 0.5)
      (bind _outactors (Actor|GetAllActorswithInterface "/Game/PairPressure/Core/Interfaces/BPI_PP_TeamMember.BPI_PP_TeamMember_C"))
      (for _array_element _outactors
        (bind _teamid (Class|BPIPPTeamMember|GetTeamId(Message) _array_element))
        (if (== _teamid (Variables|PairPressure|Tether|GetTargetTeamId))
          (if (Utilities|IsValid (Variables|PairPressure|Tether|GetEndpointA))
            (Variables|PairPressure|Tether|SetEndpointB _array_element)
            (else
              (Variables|PairPressure|Tether|SetEndpointA _array_element))))))))

(event Collision|EventActorBeginOverlap
  (params (OtherActor :type Actor%20Object%20Reference)))

(event EventTick
  (params (DeltaSeconds :type Float%20%28single-precision%29))
  (bind _endpointa (Variables|PairPressure|Tether|GetEndpointA))
  (bind _endpointb (Variables|PairPressure|Tether|GetEndpointB))
  (if (and (Utilities|IsValid _endpointa) (Utilities|IsValid _endpointb))
    (bind _anchorlocation (Class|BPIPPTetherEndpoint|GetTetherAnchor(Message) _endpointa))
    (bind _anchorlocation_2 (Class|BPIPPTetherEndpoint|GetTetherAnchor(Message) _endpointb))
    (Rendering|Debug|DrawDebugLine _anchorlocation _anchorlocation_2 "(R=0.05,G=0.75,B=1,A=1)" 0.0 5.0)
    (if (and (> (Math|Vector|VectorLength (- _anchorlocation_2 _anchorlocation)) (Variables|PairPressure|Tether|GetBreakDistance)) (not (Variables|PairPressure|Tether|GetbTetherBroken)))
      (Variables|PairPressure|Tether|SetbTetherBroken true)
      (Class|BPIPPTetherEndpoint|OnTetherBroken(Message) _endpointa)
      (Class|BPIPPTetherEndpoint|OnTetherBroken(Message) _endpointb)
      (elif (and (< (Math|Vector|VectorLength (- _anchorlocation_2 _anchorlocation)) (Variables|PairPressure|Tether|GetReconnectDistance)) (Variables|PairPressure|Tether|GetbTetherBroken))
        (Variables|PairPressure|Tether|SetbTetherBroken false)
        (Class|BPIPPTetherEndpoint|OnTetherReconnected(Message) _endpointa _endpointb)
        (Class|BPIPPTetherEndpoint|OnTetherReconnected(Message) _endpointb _endpointa)
        (elif (and (> (Math|Vector|VectorLength (- _anchorlocation_2 _anchorlocation)) (Variables|PairPressure|Tether|GetSoftLength)) (not (Variables|PairPressure|Tether|GetbTetherBroken)))
          (Class|BPIPPTetherEndpoint|ApplyTetherForce(Message) _endpointa (* (Math|Vector|Normalize (- _anchorlocation_2 _anchorlocation)) (Variables|PairPressure|Tether|GetPullStrength)))
          (Class|BPIPPTetherEndpoint|ApplyTetherForce(Message) _endpointb (Math|Vector|NegateVector (* (Math|Vector|Normalize (- _anchorlocation_2 _anchorlocation)) (Variables|PairPressure|Tether|GetPullStrength))))
          (bind _aspawn (Utilities|Casting|CastToPawn _endpointb :!pinned true)) ; Fallback direct Pawn movement retained disabled; force is delivered through BPI_PP_TetherEndpoint.
          (Pawn|Input|AddMovementInput _aspawn (Math|Vector|NegateVector (* (Math|Vector|Normalize (- _anchorlocation_2 _anchorlocation)) (Variables|PairPressure|Tether|GetPullStrength))) 1.0 false :!pinned true) ; Fallback direct Pawn movement retained disabled; force is delivered through BPI_PP_TetherEndpoint.
        )))))

(fn ConstructionScript
  (Variables|PairPressure|Tether|SetPullStrength 8.5e+04))

(fn GetTetherPresentation
  (bind _endpointa (Variables|PairPressure|Tether|GetEndpointA))
  (bind _endpointb (Variables|PairPressure|Tether|GetEndpointB))
  (bind _btetherbroken (Variables|PairPressure|Tether|GetbTetherBroken))
  (bind _anchorlocation (Class|BPIPPTetherEndpoint|GetTetherAnchor(Message) _endpointa))
  (bind _anchorlocation_2 (Class|BPIPPTetherEndpoint|GetTetherAnchor(Message) _endpointb))
  (return (Variables|PairPressure|Tether|GetTargetTeamId) (Math|Float|MapRangeClamped (Math|Vector|Distance(Vector) _anchorlocation _anchorlocation_2) (Variables|PairPressure|Tether|GetSoftLength) (Variables|PairPressure|Tether|GetBreakDistance) 0.0 1.0) (Math|Vector|Distance(Vector) _anchorlocation _anchorlocation_2) _btetherbroken (and (and (Utilities|IsValid _endpointa) (Utilities|IsValid _endpointb)) (not _btetherbroken))))